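; BP_NPC is an AI-driven non-player character that walks to a display case once the game has started.
; Each Tick it casts player character 0 to VRPawn and checks its GameStart flag.
; While the flag is set, it re-fetches a DisplayCase with GetActorOfClass and reissues an AI MoveToActor toward it every frame.
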(event Custom|MoveNPC
  (Utilities|IsValid (Variables|Default|GetTarget)
    (:Is%20Valid
      (AI|Navigation|MovetoActor (AI|GetAIController self) (Variables|Default|GetTarget) 1.0 true true true 0))))

(event EventTick
  (params (DeltaSeconds :type Float%20%28single-precision%29))
  (bind _asvrpawn (Utilities|Casting|CastToVRPawn (Game|GetPlayerCharacter 0)))
  (if (Variables|/Game/VRTemplate/Blueprints/VRPawn.VRPawn_C|GetGameStart _asvrpawn)
    (bind _returnvalue (Actor|GetActorOfClass "/Game/GameContent/DisplayCase.DisplayCase_C"))
    (Variables|Default|SetTarget _returnvalue)
    (CallFunction|MoveNPC)))

(fn ConstructionScript)